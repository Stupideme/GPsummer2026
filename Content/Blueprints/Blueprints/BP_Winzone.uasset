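; BP_Winzone is a trigger volume that ends play with a win when the player overlaps its box.
; On overlap with BP_Player, it prints a win message, ignores move input on the first player controller and adds a Winv2 widget to the viewport.
; It then casts the HUD to Timer_HUD, but the commented timer stop and display are not implemented in the live chain.
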(event OnComponentBeginOverlap(Box)
  (params (OverlappedComponent :type Primitive%20Component%20Object%20Reference) (OtherActor :type Actor%20Object%20Reference) (OtherComp :type Primitive%20Component%20Object%20Reference) (OtherBodyIndex :type Integer) (bFromSweep :type Boolean) (SweepResult :type Hit%20Result%20Structure%20%28by%20ref%29))
  ;[0.15 0.15 0.15 0.5] Winzone
  ;;[0.15 0.15 0.15 0.5] Activates on overlap
  ;;[0.15 0.15 0.15 0.5] Player its cast to
  (bind _asbp_player (Utilities|Casting|CastToBP_Player OtherActor))
  (Utilities|IsValid _asbp_player
    (:Is%20Valid
      (Development|PrintText "YOU WIN")
      ;;[0.15 0.15 0.15 0.5] Disable keyboard
      (Input|SetIgnoreMoveInput (Game|GetPlayerController 0) true)
      ;;[0.15 0.15 0.15 0.5] Place widget on screen
      (bind _returnvalue (UserInterface|CreateWidget "/Game/Blueprints/Blueprints/UI/Winv2.Winv2_C"))
      (UserInterface|Viewport|AddtoViewport _returnvalue 1)
      ;;[0.15 0.15 0.15 0.5] Stop timer and display it on widget
      (Utilities|Casting|CastToTimer_HUD (HUD|GetHUD (Game|GetPlayerController 0))))
    (:Is%20Not%20Valid
      (Development|PrintText "why no win?"))))

(fn ConstructionScript)